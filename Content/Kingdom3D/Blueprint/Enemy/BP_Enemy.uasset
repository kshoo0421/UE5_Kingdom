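; Enemy actor for Kingdom3D that drives its AI controller's Blackboard state and target from actors overlapping its detection trigger.
; CheckTarget targets the nearest detected item, or targets a wall, player or citizen and changes state, discarding other actor types.
; Any damage costs one HP; death runs a detach step for held items before destroying the enemy.
; RunAway switches the Blackboard to another state.
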(event `self.ReceiveAnyDamage`
  (params (Damage :type "Float (single-precision)") (DamageType :type "DamageType Object Reference") (InstigatedBy :type "Controller Object Reference") (DamageCauser :type "Actor Object Reference"))
  (`self.OnDamaged`))

(event `self.DetectTrigger.OnComponentBeginOverlap`
  (params (OverlappedComponent :type "PrimitiveComponent Object Reference") (OtherActor :type "Actor Object Reference") (OtherComp :type "PrimitiveComponent Object Reference") (OtherBodyIndex :type Integer) (bFromSweep :type Boolean) (SweepResult :type "HitResult Structure (by ref)"))
  (`KismetArrayLibrary.Array_Add` (`self.Detect Actors`) OtherActor))

(event `self.DetectTrigger.OnComponentEndOverlap`
  (params (OverlappedComponent :type "PrimitiveComponent Object Reference") (OtherActor :type "Actor Object Reference") (OtherComp :type "PrimitiveComponent Object Reference") (OtherBodyIndex :type Integer))
  (`KismetArrayLibrary.Array_RemoveItem` (`self.Detect Actors`) OtherActor))

(event `self.ReceiveBeginPlay`
  (bind _output_get (set `self.BB` (`AIBlueprintHelperLibrary.GetBlackboard` (`AIBlueprintHelperLibrary.GetAIController` self))))
  (`/Engine/EditorBlueprintResources/StandardMacros.IsValid` _output_get
    (:`Is Valid`
      (`BlackboardComponent.SetValueAsEnum` _output_get "state" (enumliteral `/Game/Nyeong/NY_BluePrint/Enemy/EN_EnemyState` "NewEnumerator0")))))

(fn `CheckTarget`
  (bind (_distance _returnvalue) (`GameplayStatics.FindNearestActor` (`self.K2_GetActorLocation`) (`self.Detect Actors`)))
  (`/Engine/EditorBlueprintResources/StandardMacros.IsValid` _returnvalue
    (:`Is Valid`
      (if (`GameplayStatics.ObjectIsA` _returnvalue "/Game/Kingdom3D/Blueprint/Item/BP_Item.BP_Item_C")
        (`BlackboardComponent.SetValueAsObject` (`self.BB`) "target" _returnvalue)
        (elif (or (`GameplayStatics.ObjectIsA` _returnvalue "/Game/Kingdom3D/Blueprint/Building/UpgradableBuilding/BP_Wall.BP_Wall_C") (`GameplayStatics.ObjectIsA` _returnvalue "/Game/Kingdom3D/Blueprint/Player/BP_Player.BP_Player_C") (`GameplayStatics.ObjectIsA` _returnvalue "/Game/Kingdom3D/Blueprint/Citizen/BP_Citizen.BP_Citizen_C"))
          (`BlackboardComponent.SetValueAsObject` (`self.BB`) "target" _returnvalue)
          (`BlackboardComponent.SetValueAsEnum` (`self.BB`) "state" (enumliteral `/Game/Nyeong/NY_BluePrint/Enemy/EN_EnemyState` "NewEnumerator2"))
          (else
            (`KismetArrayLibrary.Array_RemoveItem` (`self.Detect Actors`) _returnvalue)))))))

(fn `Dead`
  (if (`self.isHoldingSomething`)
    (for _array_element (`self.GetAllChildActors` self true)
      (if (`GameplayStatics.ObjectIsA` _array_element "/Game/Kingdom3D/Blueprint/Item/BP_Item.BP_Item_C")
        (`self.K2_DetachFromActor` "KeepWorld"))))
  (`self.K2_DestroyActor`))

(fn `OnDamaged`
  (bind _output_get (set `self.HP` (- (`self.HP`) 1)))
  (if (<= _output_get 0)
    (`self.Dead`)))

(fn `RunAway`
  (bind _bb (`self.BB`))
  (`/Engine/EditorBlueprintResources/StandardMacros.IsValid` _bb
    (:`Is Valid`
      (`BlackboardComponent.SetValueAsEnum` _bb "state" (enumliteral `/Game/Nyeong/NY_BluePrint/Enemy/EN_EnemyState` "NewEnumerator3")))))

(fn `UserConstructionScript`)