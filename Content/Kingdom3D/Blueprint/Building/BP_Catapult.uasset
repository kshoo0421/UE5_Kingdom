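; BP_Catapult is a catapult Blueprint among the Kingdom3D buildings, implementing only hit-point tracking and destruction.
; BeginPlay runs the parent logic, then fills CurHP from MaxHP.
; Each OnDamaged call removes one hit point and destroys the actor when CurHP equals exactly zero.
; It has no firing or targeting logic of its own, and its Tick and overlap events are disabled stubs.
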(event `self.ReceiveBeginPlay`
  (`parent.ReceiveBeginPlay`)
  (set `self.curHP` (`self.maxHP`)))

(fn `OnDamaged`
  (bind _result (`/Engine/EditorBlueprintResources/StandardMacros.DecrementInt` (`self.curHP`))
    (:`  `
      (bind _output_get (set `self.curHP` _result))
      (if (== _output_get 0)
        (`self.K2_DestroyActor`)))))

(fn `UserConstructionScript`
  (`parent.UserConstructionScript`))