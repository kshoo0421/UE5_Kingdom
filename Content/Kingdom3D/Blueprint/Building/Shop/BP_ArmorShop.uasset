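; BP_ArmorShop is a shop building where the player buys armor for five coins.
; Box overlaps feed the parent's Overlapped handler, and Interaction checks accessibility, coins and two IsArmorOn slots.
; A purchase spawns BP_Armor at the shop, offset along X by slot, and deducts the cost; failures print debug messages.
; Slots are never marked filled here, and DestroyArmor, TakeArmor, GetIsArmorOn and IsItemMax are stubs.
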(event `self.ReceiveBeginPlay`
  (`parent.ReceiveBeginPlay`))

(event `self.Box.OnComponentBeginOverlap`
  (params (OverlappedComponent :type "PrimitiveComponent Object Reference") (OtherActor :type "Actor Object Reference") (OtherComp :type "PrimitiveComponent Object Reference") (OtherBodyIndex :type Integer) (bFromSweep :type Boolean) (SweepResult :type "HitResult Structure (by ref)"))
  (`self.Overlapped` true OtherActor))

(event `self.Box.OnComponentEndOverlap`
  (params (OverlappedComponent :type "PrimitiveComponent Object Reference") (OtherActor :type "Actor Object Reference") (OtherComp :type "PrimitiveComponent Object Reference") (OtherBodyIndex :type Integer))
  (`self.Overlapped` false OtherActor))

(event `self.Interaction`
  (bind _player (`self.Player`))
  (bind _isarmoron (`self.isArmorOn`))
  (bind _coin (`/Game/Kingdom3D/Blueprint/Player/BP_Player.coin` _player))
  (if (`self.isAccessible`)
    (if (>= _coin 5)
      (if (`|GetArrayItem` _isarmoron)
        (if (`|GetArrayItem` _isarmoron 1)
          (`KismetSystemLibrary.PrintString` "Armor 생산 불가 : 공간 부족")
          (else
            (`self.ProduceArmor` 1)
            (set `/Game/Kingdom3D/Blueprint/Player/BP_Player.coin` (- _coin 5) _player :!label _label)))
        (else
          (`self.ProduceArmor` 0)
          (goto _label)))
      (else
        (`KismetSystemLibrary.PrintString` "armor 생산 불가 : 돈 부족")))
    (else
      (`KismetSystemLibrary.PrintString` "Can't Accessible"))))

(fn `DestroyArmor`
  (params (index :type Integer)))

(fn `GetIsArmorOn`
  (params (index :type Integer))
  (returns (result :type Boolean))
  (return false))

(fn `IsItemMax`
  (returns (result :type Boolean))
  (return false))

(fn `Overlapped`
  (params (IsOverlapped :type Boolean) (InputActor :type "Actor Object Reference"))
  (`parent.Overlapped` IsOverlapped InputActor))

(fn `ProduceArmor`
  (params (index :type Integer))
  (bind _returnvalue (`self.GetTransform` self))
  (`|SpawnActorFromClass` "/Game/Kingdom3D/Blueprint/Item/BP_Armor.BP_Armor_C" (`KismetMathLibrary.MakeTransform` (`KismetMathLibrary.MakeVector` (+ (.x (.location _returnvalue)) (* 20.0 index)) (.y (.location _returnvalue)) (.z (.location _returnvalue))) (.rotation _returnvalue) (.scale _returnvalue)) "Undefined" "MultiplyWithRoot" null null)
  (return))

(fn `TakeArmor`
  (params (index :type Integer)))

(fn `UserConstructionScript`
  (`parent.UserConstructionScript`))