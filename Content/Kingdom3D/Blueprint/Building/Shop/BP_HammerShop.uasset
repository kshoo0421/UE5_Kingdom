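; BP_HammerShop is a shop building where a player with enough coins can interact to produce hammers, up to a cap.
; Box overlaps feed Overlapped, and Interaction checks accessibility, coin count and the Hammers array length before calling ProduceItem.
; ProduceHammer spawns BP_Hammer actors in a row along X and stores them in Hammers.
; The purchase assigns Coin a negative constant instead of subtracting the price, and IsItemMax always returns false.
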(event `self.Box.OnComponentBeginOverlap`
  (params (OverlappedComponent :type "PrimitiveComponent Object Reference") (OtherActor :type "Actor Object Reference") (OtherComp :type "PrimitiveComponent Object Reference") (OtherBodyIndex :type Integer) (bFromSweep :type Boolean) (SweepResult :type "HitResult Structure (by ref)"))
  (`self.Overlapped` true OtherActor))

(event `self.Box.OnComponentEndOverlap`
  (params (OverlappedComponent :type "PrimitiveComponent Object Reference") (OtherActor :type "Actor Object Reference") (OtherComp :type "PrimitiveComponent Object Reference") (OtherBodyIndex :type Integer))
  (`self.Overlapped` false OtherActor))

(event `self.Interaction`
  (bind _player (`self.Player`))
  (if (`self.isAccessible`)
    (if (>= (`/Game/Kingdom3D/Blueprint/Player/BP_Player.coin` _player) 3)
      (if (<= (`KismetArrayLibrary.Array_Length` (`self.hammers`)) 4)
        (`self.ProduceItem`)
        (set `/Game/Kingdom3D/Blueprint/Player/BP_Player.coin` (- 0 3) _player)
        (else
          (`KismetSystemLibrary.PrintString` "Hammer : Max Hammer")))
      (else
        (`KismetSystemLibrary.PrintString` "Hammer : No Coin")))
    (else
      (`KismetSystemLibrary.PrintString` "Can't Accessible"))))

(event `/Game/Sihoo/SH_Blueprint/BPS_KingdomTest/Shop/BPIS_ItemShop.ProduceItem`
  (`self.ProduceHammer` 1))

(fn `IsItemMax`
  (returns (result :type Boolean))
  (return false))

(fn `ProduceHammer`
  (params (HammerCnt :type Integer))
  (bind _returnvalue (`self.GetTransform` self))
  (for _ (range 1 (+ HammerCnt 1))
    (bind _returnvalue_2 (`|SpawnActorFromClass` "/Game/Kingdom3D/Blueprint/Item/BP_Hammer.BP_Hammer_C" (`KismetMathLibrary.MakeTransform` (`KismetMathLibrary.MakeVector` (+ (.x (.location _returnvalue)) (* (`KismetArrayLibrary.Array_Length` (`self.hammers`)) 10)) (.y (.location _returnvalue)) (.z (.location _returnvalue))) (.rotation _returnvalue) (.scale _returnvalue)) "Undefined" "MultiplyWithRoot" null null))
    (`KismetArrayLibrary.Array_Add` (`self.hammers`) _returnvalue_2)))

(fn `UserConstructionScript`
  (`parent.UserConstructionScript`))