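; Building manager that lays out the kingdom's starting castle, shops and walls along the X axis at BeginPlay.
; Per-building spawn functions store references and pass initial item counts, all zero, to the bow, hammer and farmer shops.
; SpawnWalls fills the Walls array at fixed spacing; its negative-X loop is nested inside the positive-X loop, so those walls spawn repeatedly, starting at X zero.
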(event `self.ReceiveBeginPlay`
  (`self.SpawnShops`)
  (`self.SpawnWalls` 3))

(fn `SpawnArmorShop`
  (params (Xpos :type "Float (double-precision)"))
  (bind _returnvalue (`|SpawnActorFromClass` "/Game/Kingdom3D/Blueprint/Building/Shop/BP_ArmorShop.BP_ArmorShop_C" (`KismetMathLibrary.MakeTransform` (`KismetMathLibrary.MakeVector` Xpos (`self.BuildingYPos`) (`self.BuildingZPos`))) "Undefined" "MultiplyWithRoot" null null))
  (set `self.armorShop` _returnvalue))

(fn `SpawnBowShop`
  (params (XPos :type "Float (double-precision)") (BowCnt :type Integer))
  (bind _returnvalue (`|SpawnActorFromClass` "/Game/Kingdom3D/Blueprint/Building/Shop/BP_BowShop.BP_BowShop_C" (`KismetMathLibrary.MakeTransform` (`KismetMathLibrary.MakeVector` XPos (`self.BuildingYPos`) (`self.BuildingZPos`))) "Undefined" "MultiplyWithRoot" null null))
  (bind _output_get (set `self.bowShop` _returnvalue))
  (`/Game/Kingdom3D/Blueprint/Building/Shop/BP_BowShop.ProduceBow` _output_get BowCnt))

(fn `SpawnCastle`
  (params (XPos :type "Float (double-precision)"))
  (bind _returnvalue (`|SpawnActorFromClass` "/Game/Kingdom3D/Blueprint/Building/UpgradableBuilding/BP_Castle.BP_Castle_C" (`KismetMathLibrary.MakeTransform` (`KismetMathLibrary.MakeVector` XPos (`self.BuildingYPos`) (`self.BuildingZPos`))) "Undefined" "MultiplyWithRoot" null null))
  (set `self.castle` _returnvalue))

(fn `SpawnCatapultShop`
  (params (XPos :type "Float (double-precision)"))
  (bind _returnvalue (`|SpawnActorFromClass` "/Game/Kingdom3D/Blueprint/Building/Shop/BP_CatapultShop.BP_CatapultShop_C" (`KismetMathLibrary.MakeTransform` (`KismetMathLibrary.MakeVector` XPos (`self.BuildingYPos`) (`self.BuildingZPos`))) "Undefined" "MultiplyWithRoot" null null))
  (set `self.catapultShop` _returnvalue))

(fn `SpawnFarmerShop`
  (params (XPos :type "Float (double-precision)") (SytheCnt :type Integer))
  (bind _returnvalue (`|SpawnActorFromClass` "/Game/Kingdom3D/Blueprint/Building/Shop/BP_FarmerShop.BP_FarmerShop_C" (`KismetMathLibrary.MakeTransform` (`KismetMathLibrary.MakeVector` XPos (`self.BuildingYPos`) (`self.BuildingZPos`))) "Undefined" "MultiplyWithRoot" null null))
  (bind _output_get (set `self.farmerShop` _returnvalue))
  (`/Game/Kingdom3D/Blueprint/Building/Shop/BP_FarmerShop.ProduceSythe` _output_get SytheCnt))

(fn `SpawnHammerShop`
  (params (XPos :type "Float (double-precision)") (HammerCnt :type Integer))
  (bind _returnvalue (`|SpawnActorFromClass` "/Game/Kingdom3D/Blueprint/Building/Shop/BP_HammerShop.BP_HammerShop_C" (`KismetMathLibrary.MakeTransform` (`KismetMathLibrary.MakeVector` XPos (`self.BuildingYPos`) (`self.BuildingZPos`))) "Undefined" "MultiplyWithRoot" null null))
  (bind _output_get (set `self.hammerShop` _returnvalue))
  (`/Game/Kingdom3D/Blueprint/Building/Shop/BP_HammerShop.ProduceHammer` _output_get HammerCnt))

(fn `SpawnShops`
  (`self.SpawnCastle` 0.0)
  (`self.SpawnBowShop` 450.0)
  (`self.SpawnHammerShop` -450.0)
  (`self.SpawnFarmerShop` 900.0)
  (`self.SpawnArmorShop` 200.0)
  (`self.SpawnCatapultShop` -900.0))

(fn `SpawnWalls`
  (params (WallsCnt :type Integer))
  ;[1 1 1] RightWall
  (for _index (range (+ WallsCnt 1))
    (bind _returnvalue (`|SpawnActorFromClass` "/Game/Kingdom3D/Blueprint/Building/UpgradableBuilding/BP_Wall.BP_Wall_C" (`KismetMathLibrary.MakeTransform` (`KismetMathLibrary.MakeVector` (`KismetMathLibrary.Conv_IntToDouble` (* (+ _index 1) 500)) (+ (`self.BuildingYPos`) 180.0) (- (`self.BuildingZPos`) 75.0))) "Undefined" "MultiplyWithRoot" null null))
    (`KismetArrayLibrary.Array_Add` (`self.walls`) _returnvalue)
    ;[1 1 1] RightWall
    (for _index_2 (range (+ WallsCnt 1))
      (bind _returnvalue_2 (`|SpawnActorFromClass` "/Game/Kingdom3D/Blueprint/Building/UpgradableBuilding/BP_Wall.BP_Wall_C" (`KismetMathLibrary.MakeTransform` (`KismetMathLibrary.MakeVector` (`KismetMathLibrary.Conv_IntToDouble` (* _index_2 -500)) (+ (`self.BuildingYPos`) 180.0) (- (`self.BuildingZPos`) 75.0))) "Undefined" "MultiplyWithRoot" null null))
      (`KismetArrayLibrary.Array_Add` (`self.walls`) _returnvalue_2))))

(fn `UserConstructionScript`)