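; BP_Tree is an interactable tree in the Kingdom3D building set that the player pays one coin to mark.
; A Box component reports overlap begin and end, with the other actor, through Overlapped.
; Interaction checks the player's coins, deducts one, sets IsMarked and emits a "Tree"-tagged noise event at its location as a signal for AI hearing.
; Success and no-coin outcomes only print debug strings.
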(event `self.ReceiveBeginPlay`
  (`parent.ReceiveBeginPlay`))

(event `/Game/Sihoo/SH_Blueprint/BPS_KingdomTest/BPIS_IBuildingInteraction.Interaction`
  (bind _player (`self.Player`))
  (bind _coin (`/Game/Kingdom3D/Blueprint/Player/BP_Player.coin` _player))
  (if (> _coin 0)
    (bind _result (`/Engine/EditorBlueprintResources/StandardMacros.DecrementInt` _coin)
      (:`  `
        (set `/Game/Kingdom3D/Blueprint/Player/BP_Player.coin` _result _player)
        (set `self.IsMarked` true)
        (`AISense_Hearing.ReportNoiseEvent` (`self.K2_GetActorLocation`) 1.0 self 0.0 "Tree")
        (`KismetSystemLibrary.PrintString` "CallSuccessed")))
    (else
      (`KismetSystemLibrary.PrintString` "No Coin"))))

(event `self.Box.OnComponentBeginOverlap`
  (params (OverlappedComponent :type "PrimitiveComponent Object Reference") (OtherActor :type "Actor Object Reference") (OtherComp :type "PrimitiveComponent Object Reference") (OtherBodyIndex :type Integer) (bFromSweep :type Boolean) (SweepResult :type "HitResult Structure (by ref)"))
  (`self.Overlapped` true OtherActor))

(event `self.Box.OnComponentEndOverlap`
  (params (OverlappedComponent :type "PrimitiveComponent Object Reference") (OtherActor :type "Actor Object Reference") (OtherComp :type "PrimitiveComponent Object Reference") (OtherBodyIndex :type Integer))
  (`self.Overlapped` false OtherActor))

(fn `UserConstructionScript`
  (`parent.UserConstructionScript`))