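; BP_Statue is an upgradable statue building whose look changes with its level.
; Box overlap begin and end events pass the other actor to the Overlapped function.
; The Upgrade event increments CurLevel and checks it against MaxLevel, printing whether the upgrade completed or hit the cap.
; SetStatueMaterial, called on BeginPlay and successful upgrade, swaps the cube's material between two temporary castle materials by level.
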(event `self.ReceiveBeginPlay`
  (`parent.ReceiveBeginPlay`)
  (`self.SetStatueMaterial` (`self.curLevel`)))

(event `self.Box.OnComponentBeginOverlap`
  (params (OverlappedComponent :type "PrimitiveComponent Object Reference") (OtherActor :type "Actor Object Reference") (OtherComp :type "PrimitiveComponent Object Reference") (OtherBodyIndex :type Integer) (bFromSweep :type Boolean) (SweepResult :type "HitResult Structure (by ref)"))
  (`self.Overlapped` true OtherActor))

(event `self.Box.OnComponentEndOverlap`
  (params (OverlappedComponent :type "PrimitiveComponent Object Reference") (OtherActor :type "Actor Object Reference") (OtherComp :type "PrimitiveComponent Object Reference") (OtherBodyIndex :type Integer))
  (`self.Overlapped` false OtherActor))

(event `/Game/Sihoo/SH_Blueprint/BPS_KingdomTest/UpgradableBuilding/BPIS_IUpgradableBuilding.Upgrade`
  ;[1 1 1] Upgrade Event
  ;;[1 0.5 1] IsUpgradable
  (bind _result (`/Engine/EditorBlueprintResources/StandardMacros.IncrementInt` (`self.curLevel`))
    (:`  `
      (if (<= _result (`self.maxLevel`))
        ;;[1 0.5 1] Upgrade
        (bind _output_get (set `self.curLevel` _result))
        (`self.SetStatueMaterial` _output_get)
        (`KismetSystemLibrary.PrintString` "UpgradeComplete")
        (else
          ;;[1 0.5 1] Can't Upgrade
          (`KismetSystemLibrary.PrintString` "Can't Upgrade : Max Level"))))))

(fn `SetStatueMaterial`
  (params (index :type Integer))
  (bind _cube (`self.Cube`))
  (switch `int` index
    (:`Default`
      (`PrimitiveComponent.SetMaterial` _cube 0 "/Game/Kingdom3D/Material/Building/Castle/TmpCastle0.TmpCastle0" :!label _label))
    (:`0`
      (goto _label))
    (:`1`
      (`PrimitiveComponent.SetMaterial` _cube 0 "/Game/Kingdom3D/Material/Building/Castle/TmpCastle1.TmpCastle1"))))

(fn `UserConstructionScript`
  (`parent.UserConstructionScript`))