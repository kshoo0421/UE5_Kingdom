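; Upgradable building Blueprint that lets the player spend coins to raise the building's level.
; The Interaction event checks accessibility, max level and the player's coins against the current level's cost, then deducts the cost and calls Upgrade.
; Each outcome prints a debug message.
; GetIsUpgrading returns the upgrading flag, while CheckUpgradeComplete and IsMaxLevel are stubs returning false.
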(event `/Game/Sihoo/SH_Blueprint/BPS_KingdomTest/BPIS_IBuildingInteraction.Interaction`
  (bind _maxlevel (`self.maxLevel`))
  (bind _player (`self.Player`))
  (bind _output (`|GetArrayItem` (`self.upgradeCost`) (`self.curLevel`)))
  (bind _coin (`/Game/Kingdom3D/Blueprint/Player/BP_Player.coin` _player))
  ;[1 1 1] Interaction Event
  ;;[1 0.5 1] Is Accessible
  (if (`self.isAccessible`)
    ;;[1 0.5 1] Is CurLevel == MaxLevel?
    (if (!= (`self.curLevel`) _maxlevel)
      ;;[1 0.5 1] Is CurCoin >= Cost?
      (if (>= _coin _output)
        ;;[1 0.5 1] Upgrade
        (set `/Game/Kingdom3D/Blueprint/Player/BP_Player.coin` (- _coin _output) _player)
        (`/Game/Sihoo/SH_Blueprint/BPS_KingdomTest/UpgradableBuilding/BPIS_IUpgradableBuilding.Upgrade`)
        (`KismetSystemLibrary.PrintString` (`KismetTextLibrary.Conv_TextToString` (`|FormatText` "UpgradeComplete  => curLevel : {cur}" (`self.curLevel`))))
        (else
          ;;[1 0.5 1] Insufficient Coin
          (`KismetSystemLibrary.PrintString` (`KismetTextLibrary.Conv_TextToString` (`|FormatText` "curCoin is Unsufficient - cur : {cur} / cost : {cost}" _coin _output)))))
      (else
        (`KismetSystemLibrary.PrintString` (`KismetTextLibrary.Conv_TextToString` (`|FormatText` "Castle : Max Level : {MaxLevel}" _maxlevel)))))
    (else
      (`KismetSystemLibrary.PrintString` "Can't Accessible"))))

(fn `CheckUpgradeComplete`
  (returns (result :type Boolean))
  (return false))

(fn `GetIsUpgrading`
  (returns (NewParam :type Boolean))
  (return (`self.isUpgrading`)))

(fn `isMaxLevel`
  (returns (result :type Boolean))
  (return false))

(fn `UserConstructionScript`
  (`parent.UserConstructionScript`))