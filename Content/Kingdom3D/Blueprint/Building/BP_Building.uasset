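; BP_Building is a building actor that tracks whether the player can access it in Kingdom3D.
; BeginPlay caches player character 0 as a BP_Player.
; The Overlapped function sets IsAccessible for that player and registers the building as the player's current building, or clears it when the overlap ends.
; No overlap event in this graph calls Overlapped, and a debug print marks entry.
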(event `self.ReceiveBeginPlay`
  (bind _asbp_player (cast `/Game/Kingdom3D/Blueprint/Player/BP_Player` (`GameplayStatics.GetPlayerCharacter` 0)))
  (set `self.Player` _asbp_player))

(fn `Overlapped`
  (params (IsOverlapped :type Boolean) (InputActor :type "Actor Object Reference"))
  (bind _player (`self.Player`))
  (if (== InputActor _player)
    (bind _output_get (set `self.isAccessible` IsOverlapped))
    (if _output_get
      (`/Game/Kingdom3D/Blueprint/Player/BP_Player.SetCurBuilding` _player self)
      (`KismetSystemLibrary.PrintString` "Overlapped")
      (else
        (`/Game/Kingdom3D/Blueprint/Player/BP_Player.SetCurBuilding` _player null)))))

(fn `UserConstructionScript`)