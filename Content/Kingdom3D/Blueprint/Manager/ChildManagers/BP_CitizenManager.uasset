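; BP_CitizenManager is a manager Blueprint that spawns the kingdom's citizens by role: jobless, archer, carpenter, farmer and knight.
; Each role has its own spawn function, which creates the matching actor at a given location and adds it to that role's array.
; It only adds to these arrays, with no removal or role-change logic, and includes a debug TestFunc that prints a test string.
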(fn `SpawnArcher`
  (params (Location :type "Vector Structure"))
  (bind _returnvalue (`|SpawnActorFromClass` "/Game/Kingdom3D/Blueprint/Citizen/Archer/BP_Archer.BP_Archer_C" (`KismetMathLibrary.MakeTransform` Location) "Undefined" "MultiplyWithRoot" null null))
  (`KismetArrayLibrary.Array_Add` (`self.Archers`) _returnvalue)
  (return))

(fn `SpawnCarpenter`
  (params (Location :type "Vector Structure"))
  (bind _returnvalue (`|SpawnActorFromClass` "/Game/Kingdom3D/Blueprint/Citizen/Carpenter/BP_Carpenter.BP_Carpenter_C" (`KismetMathLibrary.MakeTransform` Location) "Undefined" "MultiplyWithRoot" null null))
  (`KismetArrayLibrary.Array_Add` (`self.Carpenters`) _returnvalue)
  (return))

(fn `SpawnFarmer`
  (params (Location :type "Vector Structure"))
  (bind _returnvalue (`|SpawnActorFromClass` "/Game/Kingdom3D/Blueprint/Citizen/Farmer/BP_Farmer.BP_Farmer_C" (`KismetMathLibrary.MakeTransform` Location) "Undefined" "MultiplyWithRoot" null null))
  (`KismetArrayLibrary.Array_Add` (`self.Farmers`) _returnvalue)
  (return))

(fn `SpawnJobless`
  (params (Location :type "Vector Structure"))
  (bind _returnvalue (`|SpawnActorFromClass` "/Game/Kingdom3D/Blueprint/Citizen/Jobless/BP_Jobless.BP_Jobless_C" (`KismetMathLibrary.MakeTransform` Location) "Undefined" "MultiplyWithRoot" null null))
  (`KismetArrayLibrary.Array_Add` (`self.Joblesses`) _returnvalue)
  (return))

(fn `SpawnKnights`
  (params (Location :type "Vector Structure"))
  (bind _returnvalue (`|SpawnActorFromClass` "/Game/Kingdom3D/Blueprint/Citizen/Knight/BP_Knight.BP_Knight_C" (`KismetMathLibrary.MakeTransform` Location) "Undefined" "MultiplyWithRoot" null null))
  (`KismetArrayLibrary.Array_Add` (`self.Knights`) _returnvalue)
  (return))

(fn `TestFunc`
  (`KismetSystemLibrary.PrintString` "Test"))