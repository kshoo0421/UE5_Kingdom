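; BP_EnemyManager spawns waves of enemies from alternating portals and sends them fleeing, tied to the game's day/night cycle.
; On BeginPlay it binds to the DayManager's day-start and night-start events.
; Spawning picks the left portal on even days and the right on odd, creating one enemy per day number at one-second intervals.
; Each enemy stores its spawn portal and joins a tracked array, which the retreat event loops over to call RunAway.
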(event `self.ReceiveBeginPlay`
  (bind _output_get (set `self.DayManager` (`Actor.GetComponentByClass` (`self.ManagerActor`) "/Game/Kingdom3D/Blueprint/Manager/ChildManagers/BP_DayManager.BP_DayManager_C")))
  (add `/Game/Kingdom3D/Blueprint/Manager/ChildManagers/BP_DayManager.DayStartEvent` _output_get (`|CreateDelegate` :!event `MakeEnemysRunAway`))
  (add `/Game/Kingdom3D/Blueprint/Manager/ChildManagers/BP_DayManager.NightStartEvent` _output_get (`|CreateDelegate` :!event `SpawnEnemys`)))

(event `MakeEnemysRunAway`
  (for _array_element (`self.Enemys`)
    (`/Engine/EditorBlueprintResources/StandardMacros.IsValid` _array_element
      (:`Is Valid`
        (`/Game/Kingdom3D/Blueprint/Enemy/BP_Enemy.RunAway` _array_element))))
  (`KismetSystemLibrary.PrintString` "MakeRunAway"))

(event `SpawnEnemys`
  (bind _day (`/Game/Kingdom3D/Blueprint/Manager/ChildManagers/BP_DayManager.day` (`self.DayManager`)))
  (`KismetSystemLibrary.PrintString` "SpawnEnemy")
  (if (== (mod _day 2) 0)
    (set `self.curSpawnPortal` (`self.LeftPortal`))
    (else
      (set `self.curSpawnPortal` (`self.RightPortal`))))
  (`/Game/Kingdom3D/Blueprint/Additional/ForLoopWithDelay.ForLoopWithDelay` 1 _day 1.0
    (:`LoopBody`
      (bind _returnvalue (`|SpawnActorFromClass` "/Game/Kingdom3D/Blueprint/Enemy/BP_Enemy.BP_Enemy_C" (`Actor.GetTransform` (`self.curSpawnPortal`)) "AdjustIfPossibleButAlwaysSpawn" "MultiplyWithRoot" null null))
      (set `/Game/Kingdom3D/Blueprint/Enemy/BP_Enemy.spawnPortal` (`self.curSpawnPortal`) _returnvalue)
      (`KismetArrayLibrary.Array_Add` (`self.Enemys`) _returnvalue))))