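; BP_BM2 is a building manager that spawns the kingdom's structures along the X axis when Init runs.
; SpawnShops places the castle at the origin with bow, hammer, farmer, armor and catapult shops at fixed offsets, calling the initial produce functions on the tool shops.
; SpawnUpgradableBuildings adds evenly spaced walls, farms and towers mirrored on both sides, plus one statue with a random type.
; Every spawned building is stored in a variable or array.
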(event EventInit
  (CallFunction|SpawnShops)
  (CallFunction|SpawnUpgradableBuildings))

(fn SpawnShops
  (CallFunction|SpawnCastle 0.0)
  (CallFunction|SpawnBowShop 4.5e+02)
  (CallFunction|SpawnHammerShop -4.5e+02)
  (CallFunction|SpawnFarmerShop 9e+02)
  (CallFunction|SpawnArmorShop 2e+02)
  (CallFunction|SpawnCatapultShop -9e+02))

(fn SpawnBowShop
  (params (XPos :type Float%20%28double-precision%29) (BowCnt :type Integer))
  (bind _returnvalue (Game|SpawnActorfromClass "/Game/Kingdom3D/Blueprint/Building/Shop/BP_BowShop.BP_BowShop_C" (Math|Transform|MakeTransform (Math|Vector|MakeVector XPos (Utilities|BuildingYPos) (Utilities|BuildingZPos)) "0, 0, 0" "1.000000,1.000000,1.000000") "Undefined" "MultiplyWithRoot" 0 0))
  (bind _output_get (Variables|Default|SetbowShop _returnvalue))
  (Default|ProduceBow _output_get BowCnt))

(fn SpawnArmorShop
  (params (Xpo :type Float%20%28double-precision%29))
  (bind _returnvalue (Game|SpawnActorfromClass "/Game/Kingdom3D/Blueprint/Building/Shop/BP_ArmorShop.BP_ArmorShop_C" (Math|Transform|MakeTransform (Math|Vector|MakeVector Xpo (Utilities|BuildingYPos) (Utilities|BuildingZPos)) "0, 0, 0" "1.000000,1.000000,1.000000") "Undefined" "MultiplyWithRoot" 0 0))
  (Variables|Default|SetarmorShop _returnvalue))

(fn SpawnCatapultShop
  (params (XPos :type Float%20%28double-precision%29))
  (bind _returnvalue (Game|SpawnActorfromClass "/Game/Kingdom3D/Blueprint/Building/Shop/BP_CatapultShop.BP_CatapultShop_C" (Math|Transform|MakeTransform (Math|Vector|MakeVector XPos (Utilities|BuildingYPos) (Utilities|BuildingZPos)) "0, 0, 0" "1.000000,1.000000,1.000000") "Undefined" "MultiplyWithRoot" 0 0))
  (Variables|Default|SetcatapultShop _returnvalue))

(fn SpawnFarmerShop
  (params (XPos :type Float%20%28double-precision%29) (SytheCnt :type Integer))
  (bind _returnvalue (Game|SpawnActorfromClass "/Game/Kingdom3D/Blueprint/Building/Shop/BP_FarmerShop.BP_FarmerShop_C" (Math|Transform|MakeTransform (Math|Vector|MakeVector XPos (Utilities|BuildingYPos) (Utilities|BuildingZPos)) "0, 0, 0" "1.000000,1.000000,1.000000") "Undefined" "MultiplyWithRoot" 0 0))
  (bind _output_get (Variables|Default|SetfarmerShop _returnvalue))
  (Default|ProduceSythe _output_get SytheCnt))

(fn SpawnHammerShop
  (params (XPos :type Float%20%28double-precision%29) (HammerCnt :type Integer))
  (bind _returnvalue (Game|SpawnActorfromClass "/Game/Kingdom3D/Blueprint/Building/Shop/BP_HammerShop.BP_HammerShop_C" (Math|Transform|MakeTransform (Math|Vector|MakeVector XPos (Utilities|BuildingYPos) (Utilities|BuildingZPos)) "0, 0, 0" "1.000000,1.000000,1.000000") "Undefined" "MultiplyWithRoot" 0 0))
  (bind _output_get (Variables|Default|SethammerShop _returnvalue))
  (Default|ProduceHammer _output_get HammerCnt))

(fn SpawnCastle
  (params (XPos :type Float%20%28double-precision%29))
  (bind _returnvalue (Game|SpawnActorfromClass "/Game/Kingdom3D/Blueprint/Building/UpgradableBuilding/BP_Castle.BP_Castle_C" (Math|Transform|MakeTransform (Math|Vector|MakeVector XPos (Utilities|BuildingYPos) (Utilities|BuildingZPos)) "0, 0, 0" "1.000000,1.000000,1.000000") "Undefined" "MultiplyWithRoot" 0 0))
  (Variables|Default|Setcastle _returnvalue))

(fn SpawnWalls
  (params (WallCnt :type Integer))
  ;[1 1 1] RightWall
  (for _index (range 0 WallCnt)
    (bind _returnvalue (Game|SpawnActorfromClass "/Game/Kingdom3D/Blueprint/Building/UpgradableBuilding/BP_Wall.BP_Wall_C" (Math|Transform|MakeTransform (Math|Vector|MakeVector (Math|Conversions|ToFloat(Integer) (* (+ _index 1) 500)) (+ (Utilities|BuildingYPos) 1.8e+02) (- (Utilities|BuildingZPos) 75.0)) "0, 0, 0" "1.000000,1.000000,1.000000") "Undefined" "MultiplyWithRoot" 0 0))
    (Utilities|Array|Add (Variables|Default|Getwalls) _returnvalue))
  ;[1 1 1] RightWall
  (for _index_2 (range 0 WallCnt)
    (bind _returnvalue_2 (Game|SpawnActorfromClass "/Game/Kingdom3D/Blueprint/Building/UpgradableBuilding/BP_Wall.BP_Wall_C" (Math|Transform|MakeTransform (Math|Vector|MakeVector (Math|Conversions|ToFloat(Integer) (* (+ _index_2 1) -500)) (+ (Utilities|BuildingYPos) 1.8e+02) (- (Utilities|BuildingZPos) 75.0)) "0, 0, 0" "1.000000,1.000000,1.000000") "Undefined" "MultiplyWithRoot" 0 0))
    (Utilities|Array|Add (Variables|Default|Getwalls) _returnvalue_2)))

(fn SpawnFarms
  (params (FarmCnt :type Integer))
  (bind _ypos (Utilities|BuildingYPos))
  (bind _zpos (Utilities|BuildingZPos))
  (bind _returnvalue (+ _ypos 3e+02))
  (for _index (range 0 FarmCnt)
    (bind _returnvalue_2 (Game|SpawnActorfromClass "/Game/Kingdom3D/Blueprint/Building/UpgradableBuilding/BP_Farm.BP_Farm_C" (Math|Transform|MakeTransform (Math|Vector|MakeVector (|((index*1000)+1500) (Math|Conversions|ToFloat(Integer) _index)) _returnvalue _zpos) "0, 0, 0" "1.000000,1.000000,1.000000") "Undefined" "MultiplyWithRoot" 0 0))
    (Utilities|Array|Add (Variables|Default|GetFarms) _returnvalue_2)
    (bind _returnvalue_3 (Game|SpawnActorfromClass "/Game/Kingdom3D/Blueprint/Building/UpgradableBuilding/BP_Farm.BP_Farm_C" (Math|Transform|MakeTransform (Math|Vector|MakeVector (* (|((index*1000)+1500) (Math|Conversions|ToFloat(Integer) _index)) -1.0) _returnvalue _zpos) "0, 0, 0" "1.000000,1.000000,1.000000") "Undefined" "MultiplyWithRoot" 0 0))
    (Utilities|Array|Add (Variables|Default|GetFarms) _returnvalue_3)))

(fn SpawnStatue
  (bind _returnvalue (Game|SpawnActorfromClass "/Game/Kingdom3D/Blueprint/Building/UpgradableBuilding/BP_Statue.BP_Statue_C" (Math|Transform|MakeTransform (Math|Vector|MakeVector 1e+03 (Utilities|BuildingYPos) (Utilities|BuildingZPos)) "0, 0, 0" "1.000000,1.000000,1.000000") "Undefined" "MultiplyWithRoot" 0 0))
  (bind _output_get (Variables|Default|Setstatue _returnvalue))
  (switch int (Math|Random|RandomInteger 4)
    (:Default
      (Variables|/Game/Kingdom3D/Blueprint/Building/UpgradableBuilding/BP_Statue.BP_Statue_C|SetstatueType _output_get "NewEnumerator2" :!label _label))
    (:0
      (goto _label))
    (:1
      (Variables|/Game/Kingdom3D/Blueprint/Building/UpgradableBuilding/BP_Statue.BP_Statue_C|SetstatueType _output_get "NewEnumerator3"))
    (:2
      (Variables|/Game/Kingdom3D/Blueprint/Building/UpgradableBuilding/BP_Statue.BP_Statue_C|SetstatueType _output_get "NewEnumerator4"))
    (:3
      (Variables|/Game/Kingdom3D/Blueprint/Building/UpgradableBuilding/BP_Statue.BP_Statue_C|SetstatueType _output_get "NewEnumerator5"))))

(fn SpawnUpgradableBuildings
  (CallFunction|SpawnWalls 4)
  (CallFunction|SpawnFarms 2)
  (CallFunction|SpawnStatue)
  (CallFunction|SpawnTowers 3))

(fn SpawnTowers
  (params (TowerCnt :type Integer))
  (bind _ypos (Utilities|BuildingYPos))
  (bind _zpos (Utilities|BuildingZPos))
  (for _index (range 0 TowerCnt)
    (bind _returnvalue (Game|SpawnActorfromClass "/Game/Kingdom3D/Blueprint/Building/UpgradableBuilding/BP_Tower.BP_Tower_C" (Math|Transform|MakeTransform (Math|Vector|MakeVector (|((index*700)+800) (Math|Conversions|ToFloat(Integer) _index)) _ypos _zpos) "0, 0, 0" "1.000000,1.000000,1.000000") "Undefined" "MultiplyWithRoot" 0 0))
    (Utilities|Array|Add (Variables|Default|GetTowers) _returnvalue)
    (bind _returnvalue_2 (Game|SpawnActorfromClass "/Game/Kingdom3D/Blueprint/Building/UpgradableBuilding/BP_Tower.BP_Tower_C" (Math|Transform|MakeTransform (Math|Vector|MakeVector (* (|((index*700)+800) (Math|Conversions|ToFloat(Integer) _index)) -1.0) _ypos _zpos) "0, 0, 0" "1.000000,1.000000,1.000000") "Undefined" "MultiplyWithRoot" 0 0))
    (Utilities|Array|Add (Variables|Default|GetTowers) _returnvalue_2)))

(fn Init
  (CallFunction|SpawnShops)
  (CallFunction|SpawnUpgradableBuildings))