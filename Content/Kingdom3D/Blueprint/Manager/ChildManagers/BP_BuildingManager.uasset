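; Building manager for the Kingdom3D level that spawns and keeps references to every building when play begins.
; SetAllBuildings first places the castle and the bow, hammer, farmer, armor and catapult shops at fixed X positions.
; It then spawns walls, farms and towers at index-spaced offsets mirrored on both sides of the origin, storing them in arrays.
; A single statue is also spawned and given a random type.
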(event EventBeginPlay
  (CallFunction|SetAllBuildings))

(event EventTick
  (params (DeltaSeconds :type Float%20%28single-precision%29)))

(fn SpawnShops
  (CallFunction|SpawnCastle)
  (CallFunction|SpawnBowShop 4.5e+02)
  (CallFunction|SpawnHammerShop -4.5e+02)
  (CallFunction|SpawnFarmerShop 9e+02)
  (CallFunction|SpawnArmorShop 2e+02)
  (CallFunction|SpawnCatapultShop -9e+02))

(fn SpawnBowShop
  (params (XPos :type Float%20%28double-precision%29) (BowCnt :type Integer))
  (bind (_x_default _y_default _z_default) (Utilities|BuildingPos))
  (bind _returnvalue (Game|SpawnActorfromClass "/Game/Kingdom3D/Blueprint/Building/Shop/BP_BowShop.BP_BowShop_C" (Math|Transform|MakeTransform (Math|Vector|MakeVector XPos _y_default _z_default) "0, 0, 0" "1.000000,1.000000,1.000000") "Undefined" "MultiplyWithRoot" 0 0))
  (bind _output_get (Variables|Default|SetbowShop _returnvalue))
  (Default|ProduceBow _output_get BowCnt))

(fn SpawnArmorShop
  (params (XPos :type Float%20%28double-precision%29))
  (bind (_x_default _y_default _z_default) (Utilities|BuildingPos))
  (bind _returnvalue (Game|SpawnActorfromClass "/Game/Kingdom3D/Blueprint/Building/Shop/BP_ArmorShop.BP_ArmorShop_C" (Math|Transform|MakeTransform (Math|Vector|MakeVector XPos _y_default _z_default) "0, 0, 0" "1.000000,1.000000,1.000000") "Undefined" "MultiplyWithRoot" 0 0))
  (Variables|Default|SetarmorShop _returnvalue))

(fn SpawnCatapultShop
  (params (XPos :type Float%20%28double-precision%29))
  (bind (_x_default _y_default _z_default) (Utilities|BuildingPos))
  (bind _returnvalue (Game|SpawnActorfromClass "/Game/Kingdom3D/Blueprint/Building/Shop/BP_CatapultShop.BP_CatapultShop_C" (Math|Transform|MakeTransform (Math|Vector|MakeVector XPos _y_default _z_default) "0, 0, 0" "1.000000,1.000000,1.000000") "Undefined" "MultiplyWithRoot" 0 0))
  (Variables|Default|SetcatapultShop _returnvalue))

(fn SpawnFarmerShop
  (params (XPos :type Float%20%28double-precision%29))
  (bind (_x_default _y_default _z_default) (Utilities|BuildingPos))
  (bind _returnvalue (Game|SpawnActorfromClass "/Game/Kingdom3D/Blueprint/Building/Shop/BP_FarmerShop.BP_FarmerShop_C" (Math|Transform|MakeTransform (Math|Vector|MakeVector XPos _y_default _z_default) "0, 0, 0" "1.000000,1.000000,1.000000") "Undefined" "MultiplyWithRoot" 0 0))
  (bind _output_get (Variables|Default|SetfarmerShop _returnvalue))
  (Default|ProduceSythe _output_get))

(fn SpawnHammerShop
  (params (XPos :type Float%20%28double-precision%29))
  (bind (_x_default _y_default _z_default) (Utilities|BuildingPos))
  (bind _returnvalue (Game|SpawnActorfromClass "/Game/Kingdom3D/Blueprint/Building/Shop/BP_HammerShop.BP_HammerShop_C" (Math|Transform|MakeTransform (Math|Vector|MakeVector XPos _y_default _z_default) "0, 0, 0" "1.000000,1.000000,1.000000") "Undefined" "MultiplyWithRoot" 0 0))
  (bind _output_get (Variables|Default|SethammerShop _returnvalue))
  (Default|ProduceHammer _output_get))

(fn SpawnUpgradableBuilding
  (CallFunction|SpawnWalls 4)
  (CallFunction|SpawnFarms 2)
  (CallFunction|SpawnStatue)
  (CallFunction|SpawnTowers 3))

(fn SpawnCastle
  (bind (_x_default _y_default _z_default) (Utilities|BuildingPos))
  (bind _returnvalue (Game|SpawnActorfromClass "/Game/Kingdom3D/Blueprint/Building/UpgradableBuilding/BP_Castle.BP_Castle_C" (Math|Transform|MakeTransform (Math|Vector|MakeVector _x_default _y_default _z_default) "0, 0, 0" "1.000000,1.000000,1.000000") "Undefined" "MultiplyWithRoot" 0 0))
  (Variables|Default|Setcastle _returnvalue))

(fn SpawnWalls
  (params (Wall%20Cnt :type Integer))
  (bind (_x_default _y_default _z_default) (Utilities|BuildingPos))
  (bind (_x_default_2 _y_default_2 _z_default_2) (Utilities|BuildingPos))
  ;[1 1 1] RightWall
  (for _index (range 0 Wall%20Cnt)
    (bind _returnvalue (Game|SpawnActorfromClass "/Game/Kingdom3D/Blueprint/Building/UpgradableBuilding/BP_Wall.BP_Wall_C" (Math|Transform|MakeTransform (Math|Vector|MakeVector (Math|Conversions|ToFloat(Integer) (* (+ _index 1) 500)) (+ _y_default 1.8e+02) (- _z_default 75.0)) "0, 0, 0" "1.000000,1.000000,1.000000") "Undefined" "MultiplyWithRoot" 0 0))
    (Utilities|Array|Add (Variables|Default|Getwalls) _returnvalue))
  ;[1 1 1] RightWall
  (for _index_2 (range 0 Wall%20Cnt)
    (bind _returnvalue_2 (Game|SpawnActorfromClass "/Game/Kingdom3D/Blueprint/Building/UpgradableBuilding/BP_Wall.BP_Wall_C" (Math|Transform|MakeTransform (Math|Vector|MakeVector (Math|Conversions|ToFloat(Integer) (* (+ _index_2 1) -500)) (+ _y_default_2 1.8e+02) (- _z_default_2 75.0)) "0, 0, 0" "1.000000,1.000000,1.000000") "Undefined" "MultiplyWithRoot" 0 0))
    (Utilities|Array|Add (Variables|Default|Getwalls) _returnvalue_2)))

(fn SpawnFarms
  (params (Farm%20Cnt :type Integer))
  (bind (_x_default _y_default _z_default) (Utilities|BuildingPos))
  (bind _returnvalue (+ _y_default 3e+02))
  (for _index (range 0 Farm%20Cnt)
    (bind _returnvalue_2 (Game|SpawnActorfromClass "/Game/Kingdom3D/Blueprint/Building/UpgradableBuilding/BP_Farm.BP_Farm_C" (Math|Transform|MakeTransform (Math|Vector|MakeVector (|((index*1000)+1500) (Math|Conversions|ToFloat(Integer) _index)) _returnvalue _z_default) "0, 0, 0" "1.000000,1.000000,1.000000") "Undefined" "MultiplyWithRoot" 0 0))
    (Utilities|Array|Add (Variables|Default|GetFarms) _returnvalue_2)
    (bind _returnvalue_3 (Game|SpawnActorfromClass "/Game/Kingdom3D/Blueprint/Building/UpgradableBuilding/BP_Farm.BP_Farm_C" (Math|Transform|MakeTransform (Math|Vector|MakeVector (* (|((index*1000)+1500) (Math|Conversions|ToFloat(Integer) _index)) -1.0) _returnvalue _z_default) "0, 0, 0" "1.000000,1.000000,1.000000") "Undefined" "MultiplyWithRoot" 0 0))
    (Utilities|Array|Add (Variables|Default|GetFarms) _returnvalue_3)))

(fn SpawnStatue
  (bind (_x_default _y_default _z_default) (Utilities|BuildingPos))
  (bind _returnvalue (Game|SpawnActorfromClass "/Game/Kingdom3D/Blueprint/Building/UpgradableBuilding/BP_Statue.BP_Statue_C" (Math|Transform|MakeTransform (Math|Vector|MakeVector 1e+03 _y_default _z_default) "0, 0, 0" "1.000000,1.000000,1.000000") "Undefined" "MultiplyWithRoot" 0 0))
  (bind _output_get (Variables|Default|Setstatue _returnvalue))
  (switch int (Math|Random|RandomInteger 4)
    (:Default
      (Variables|/Game/Kingdom3D/Blueprint/Building/UpgradableBuilding/BP_Statue.BP_Statue_C|SetstatueType _output_get "NewEnumerator2" :!label _label))
    (:0
      (goto _label))
    (:1
      (Variables|/Game/Kingdom3D/Blueprint/Building/UpgradableBuilding/BP_Statue.BP_Statue_C|SetstatueType _output_get "NewEnumerator3"))
    (:2
      (Variables|/Game/Kingdom3D/Blueprint/Building/UpgradableBuilding/BP_Statue.BP_Statue_C|SetstatueType _output_get "NewEnumerator4"))
    (:3
      (Variables|/Game/Kingdom3D/Blueprint/Building/UpgradableBuilding/BP_Statue.BP_Statue_C|SetstatueType _output_get "NewEnumerator5"))))

(fn SpawnTowers
  (params (TowerCnt :type Integer))
  (bind (_x_default _y_default _z_default) (Utilities|BuildingPos))
  (for _index (range 0 TowerCnt)
    (bind _returnvalue (Game|SpawnActorfromClass "/Game/Kingdom3D/Blueprint/Building/UpgradableBuilding/BP_Tower.BP_Tower_C" (Math|Transform|MakeTransform (Math|Vector|MakeVector (|((index*700)+800) (Math|Conversions|ToFloat(Integer) _index)) _y_default _z_default) "0, 0, 0" "1.000000,1.000000,1.000000") "Undefined" "MultiplyWithRoot" 0 0))
    (Utilities|Array|Add (Variables|Default|GetTowers) _returnvalue)
    (bind _returnvalue_2 (Game|SpawnActorfromClass "/Game/Kingdom3D/Blueprint/Building/UpgradableBuilding/BP_Tower.BP_Tower_C" (Math|Transform|MakeTransform (Math|Vector|MakeVector (* (|((index*700)+800) (Math|Conversions|ToFloat(Integer) _index)) -1.0) _y_default _z_default) "0, 0, 0" "1.000000,1.000000,1.000000") "Undefined" "MultiplyWithRoot" 0 0))
    (Utilities|Array|Add (Variables|Default|GetTowers) _returnvalue_2)))

(fn SetAllBuildings
  (CallFunction|SpawnShops)
  (CallFunction|SpawnUpgradableBuilding))