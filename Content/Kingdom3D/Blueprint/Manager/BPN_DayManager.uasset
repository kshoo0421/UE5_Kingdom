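; Day manager for Kingdom3D that drives the cycle of Day, Night and Blood Moon states and counts days.
; Tick accumulates time and switches state at the day and night length thresholds, resetting the timer only at day start.
; Every fifth day's night becomes a Blood Moon, sharing the regular night logic.
; Transitions fire day or night start events, with BeginPlay firing day start twice; per-phase tick functions are empty stubs.
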(event `self.ReceiveTick`
  (params (DeltaSeconds :type "Float (single-precision)"))
  (set `self.time` (+ DeltaSeconds (`self.time`)))
  (switch `/Game/Kingdom3D/Blueprint/Manager/EN_DayState` (`self.dayState`)
    (:`NewEnumerator0`
      (if (>= (`self.time`) (`self.dayLength`))
        (`self.NightStart`)
        (else
          (`self.DayTick`))))
    (:`NewEnumerator1`
      (if (>= (`self.time`) (`self.nightLength`)) :!label _label
        (`self.DayStart`)
        (else
          (`self.NightTick`))))
    (:`NewEnumerator2`
      (goto _label))))

(event `self.ReceiveBeginPlay`
  (`self.Initialize`))

(fn `DayStart`
  (`KismetSystemLibrary.PrintString` "Day")
  (set `self.time` 0.0)
  (set `self.dayState` "NewEnumerator0")
  (set `self.day` (+ (`self.day`) 1))
  (`self.DayStartEvent`))

(fn `DayTick`)

(fn `Initialize`
  (`self.DayStart`)
  (`self.DayStartEvent`))

(fn `NightStart`
  (if (== (mod (`self.day`) 5) 0)
    (set `self.dayState` "NewEnumerator2")
    (`KismetSystemLibrary.PrintString` "Blood Moon")
    (else
      (set `self.dayState` "NewEnumerator1")
      (`KismetSystemLibrary.PrintString` "Night")))
  (`self.NightStartEvent`))

(fn `NightTick`)