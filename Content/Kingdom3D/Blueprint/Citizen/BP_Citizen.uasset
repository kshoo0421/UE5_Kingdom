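; Citizen character for Kingdom3D that holds a job, a state and a coin count that acts as its health.
; Each damage event removes a coin, and the citizen is destroyed when the count hits -1.
; DropCoin spawns a coin offset along X by the sign of its world X.
; Helpers set walk and crouch speeds, or replace the citizen with an AI-controlled BP_Jobless running BT_Citizen.
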(event `/Game/Sihoo/SH_Blueprint/BPS_KingdomTest/Citizen/BPIS_Citizen.OnDamaged`
  ;[1 1 1] Event OnDamaged
  ;;[1 0.5 1] Coin--
  (bind _result (`/Engine/EditorBlueprintResources/StandardMacros.DecrementInt` (`self.curCoin`))
    (:`  `
      ;;[1 0.5 1] If No Coin
      (bind _output_get (set `self.curCoin` _result))
      (if (== _output_get -1)
        ;;[1 0.5 1] Destroy Citizen
        (`self.K2_DestroyActor`)
        (`KismetSystemLibrary.PrintString` "BP_Citizen : Destroyed")
        (else
          (`KismetSystemLibrary.PrintString` "OnDamaged"))))))

(fn `Drop Coin`
  (bind _returnvalue (`self.GetTransform` self))
  ;[1 1 1] If Character has Coin : Drop Coin
  ;;[1 0.5 1] Coin--
  (`/Engine/EditorBlueprintResources/StandardMacros.DecrementInt` (`self.curCoin`)
    (:`  `
      ;;[1 0.5 1] Right Or Left
      (if (> (.x (.location _returnvalue)) 0.0)
        ;;[1 0.5 1] Coin Location : Right
        (`|SpawnActorFromClass` "/Game/Kingdom3D/Blueprint/Item/BP_Coin.BP_Coin_C" (`KismetMathLibrary.MakeTransform` (`KismetMathLibrary.MakeVector` (+ (.x (.location _returnvalue)) 20.0) (.y (.location _returnvalue)) (.z (.location _returnvalue))) (.rotation _returnvalue) (.scale _returnvalue)) "Undefined" "MultiplyWithRoot" null null)
        (else
          ;;[1 0.5 1] Coin : Left
          (`|SpawnActorFromClass` "/Game/Kingdom3D/Blueprint/Item/BP_Coin.BP_Coin_C" (`KismetMathLibrary.MakeTransform` (`KismetMathLibrary.MakeVector` (- (.x (.location _returnvalue)) 20.0) (.y (.location _returnvalue)) (.z (.location _returnvalue))) (.rotation _returnvalue) (.scale _returnvalue)) "Undefined" "MultiplyWithRoot" null null)))
      (return))))

(fn `GetCitizenState`
  (returns (result :type "/Game/Kingdom3D/Blueprint/Citizen/BPE_CitizenState Enum"))
  (return (`self.citizenState`)))

(fn `GetJob`
  (returns (result :type "/Game/Kingdom3D/Blueprint/Citizen/BPE_Job Enum"))
  (return (`self.job`)))

(fn `SetMaxWalkSpeed`
  (params (`Max Walk Speed` :type "Float (single-precision)"))
  (bind _charactermovement (`self.CharacterMovement`))
  (bind _output_get (set `CharacterMovementComponent.MaxWalkSpeed` `Max Walk Speed` _charactermovement))
  (set `CharacterMovementComponent.MaxWalkSpeedCrouched` (/ _output_get 2.0) _charactermovement))

(fn `SpawnJoblessInsteadSelf`
  (bind (_returnvalue_location _returnvalue_rotation) (`KismetMathLibrary.BreakTransform` (`self.GetTransform` self)))
  ;[1 1 1] Spawn Jobless & Destroy Self
  ;;[1 0.5 1] Spawn Jobless
  (`AIBlueprintHelperLibrary.SpawnAIFromClass` "/Game/Kingdom3D/Blueprint/Citizen/Jobless/BP_Jobless.BP_Jobless_C" "/Game/Kingdom3D/Blueprint/Citizen/AI/BT_Citizen.BT_Citizen" _returnvalue_location _returnvalue_rotation false null)
  ;;[1 0.5 1] Destroy Self
  (`self.K2_DestroyActor`)
  (return))

(fn `UserConstructionScript`)