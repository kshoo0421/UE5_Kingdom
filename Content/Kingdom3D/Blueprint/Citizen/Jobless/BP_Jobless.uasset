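; BP_Jobless is the unemployed citizen pawn, which collects coins and takes a job from a picked-up tool.
; On start it registers itself and its job with AI_Citizen and the blackboard.
; Collision overlaps bank coins or swap the pawn for an Archer, Knight, Carpenter or Farmer by item type, via SpawnAIFromClass and destroy.
; Damage drops a coin away from world X zero, or turns a coinless pawn into a Wanderer.
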(event `self.ReceiveBeginPlay`
  (`parent.ReceiveBeginPlay`)
  (`KismetSystemLibrary.Delay` 0.1)
  (`self.SetAIJob`))

(event `self.Collision.OnComponentBeginOverlap`
  (params (OverlappedComponent :type "PrimitiveComponent Object Reference") (OtherActor :type "Actor Object Reference") (OtherComp :type "PrimitiveComponent Object Reference") (OtherBodyIndex :type Integer) (bFromSweep :type Boolean) (SweepResult :type "HitResult Structure (by ref)"))
  (bind _asbp_coin (cast `/Game/Kingdom3D/Blueprint/Item/BP_Coin` OtherActor)
    (:`then`
      (`self.GetCoin` _asbp_coin))
    (:`CastFailed`
      (bind _asbp_item (cast `/Game/Kingdom3D/Blueprint/Item/BP_Item` OtherActor))
      (`self.ChangeJobs` _asbp_item))))

(event `/Game/Sihoo/SH_Blueprint/BPS_KingdomTest/Citizen/BPIS_Citizen.OnDamaged`
  (`self.MinusCoin`))

(event `self.ReceiveAnyDamage`
  (params (Damage :type "Float (single-precision)") (DamageType :type "DamageType Object Reference") (InstigatedBy :type "Controller Object Reference") (DamageCauser :type "Actor Object Reference"))
  (`/Game/Sihoo/SH_Blueprint/BPS_KingdomTest/Citizen/BPIS_Citizen.OnDamaged`))

(fn `ChangeJobs`
  (params (Item :type "/Game/Kingdom3D/Blueprint/Item/BP_Item Object Reference"))
  (bind (_returnvalue_location _returnvalue_rotation) (`KismetMathLibrary.BreakTransform` (`self.GetTransform` self)))
  (cast `/Game/Kingdom3D/Blueprint/Item/BP_Bow` Item
    (:`then`
      (`AIBlueprintHelperLibrary.SpawnAIFromClass` "/Game/Kingdom3D/Blueprint/Citizen/Archer/BP_Archer.BP_Archer_C" "/Game/Kingdom3D/Blueprint/Citizen/AI/BT_Citizen.BT_Citizen" _returnvalue_location _returnvalue_rotation false null)
      (`self.K2_DestroyActor` :!label _label)
      (`self.K2_DestroyActor` Item))
    (:`CastFailed`
      (cast `/Game/Kingdom3D/Blueprint/Item/BP_Armor` Item
        (:`then`
          (`AIBlueprintHelperLibrary.SpawnAIFromClass` "/Game/Kingdom3D/Blueprint/Citizen/Knight/BP_Knight.BP_Knight_C" "/Game/Kingdom3D/Blueprint/Citizen/AI/BT_Citizen.BT_Citizen" _returnvalue_location _returnvalue_rotation false null)
          (goto _label))
        (:`CastFailed`
          (cast `/Game/Kingdom3D/Blueprint/Item/BP_Hammer` Item
            (:`then`
              (`AIBlueprintHelperLibrary.SpawnAIFromClass` "/Game/Kingdom3D/Blueprint/Citizen/Carpenter/BP_Carpenter.BP_Carpenter_C" "/Game/Kingdom3D/Blueprint/Citizen/AI/BT_Citizen.BT_Citizen" _returnvalue_location _returnvalue_rotation false null)
              (goto _label))
            (:`CastFailed`
              (cast `/Game/Kingdom3D/Blueprint/Item/BP_Sythe` Item
                (:`then`
                  (`AIBlueprintHelperLibrary.SpawnAIFromClass` "/Game/Kingdom3D/Blueprint/Citizen/Farmer/BP_Farmer.BP_Farmer_C" "/Game/Kingdom3D/Blueprint/Citizen/AI/BT_Citizen.BT_Citizen" _returnvalue_location _returnvalue_rotation false null)
                  (goto _label))
                (:`CastFailed`
                  (`KismetSystemLibrary.PrintString` "Error"))))))))))

(fn `GetCoin`
  (params (Coin :type "/Game/Kingdom3D/Blueprint/Item/BP_Coin Object Reference"))
  (`/Engine/EditorBlueprintResources/StandardMacros.IncrementInt` (`self.curCoin`)
    (:`  `
      (`self.K2_DestroyActor` Coin)
      (return))))

(fn `MinusCoin`
  (bind _curcoin (`self.curCoin`))
  (bind _returnvalue (`self.GetTransform` self))
  (bind (_returnvalue_location _returnvalue_rotation) (`KismetMathLibrary.BreakTransform` (`self.GetTransform` self)))
  (if (> _curcoin 0)
    (`/Engine/EditorBlueprintResources/StandardMacros.DecrementInt` _curcoin
      (:`  `
        (if (> (.x (.location _returnvalue)) 0.0)
          (`|SpawnActorFromClass` "/Game/Kingdom3D/Blueprint/Item/BP_Coin.BP_Coin_C" (`KismetMathLibrary.MakeTransform` (`KismetMathLibrary.MakeVector` (+ (.x (.location _returnvalue)) 20.0) (.y (.location _returnvalue)) (.z (.location _returnvalue))) (.rotation _returnvalue) (.scale _returnvalue)) "Undefined" "MultiplyWithRoot" null null)
          (else
            (`|SpawnActorFromClass` "/Game/Kingdom3D/Blueprint/Item/BP_Coin.BP_Coin_C" (`KismetMathLibrary.MakeTransform` (`KismetMathLibrary.MakeVector` (- (.x (.location _returnvalue)) 20.0) (.y (.location _returnvalue)) (.z (.location _returnvalue))) (.rotation _returnvalue) (.scale _returnvalue)) "Undefined" "MultiplyWithRoot" null null)))
        (return)))
    (else
      (`AIBlueprintHelperLibrary.SpawnAIFromClass` "/Game/Kingdom3D/Blueprint/Citizen/Wanderer/BP_Wanderer.BP_Wanderer_C" "/Game/Kingdom3D/Blueprint/Citizen/AI/BT_Citizen.BT_Citizen" _returnvalue_location _returnvalue_rotation false null)
      (`self.K2_DestroyActor`)
      (return))))

(fn `SetAIJob`
  (bind _asai_citizen (cast `/Game/Kingdom3D/Blueprint/Citizen/AI/AI_Citizen` (`AIBlueprintHelperLibrary.GetAIController` self))
    (:`then`
      (set `/Game/Kingdom3D/Blueprint/Citizen/AI/AI_Citizen.Jobless` self _asai_citizen)
      (bind _output_get (set `/Game/Kingdom3D/Blueprint/Citizen/AI/AI_Citizen.Job` "NewEnumerator1" _asai_citizen))
      (`BlackboardComponent.SetValueAsEnum` (`AIController.Blackboard` _asai_citizen) "Job" _output_get))
    (:`CastFailed`
      (`KismetSystemLibrary.PrintString` "CastFailed"))))

(fn `UserConstructionScript`
  (`parent.UserConstructionScript`))