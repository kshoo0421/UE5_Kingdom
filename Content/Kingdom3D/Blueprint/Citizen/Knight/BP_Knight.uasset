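; Knight citizen that fights enemies and loses coins when hit.
; Shortly after BeginPlay it registers itself and its job with AI_Citizen and the blackboard.
; AttackRange overlaps store the enemy and mirror its HP to the blackboard, while Attack_Event damages that enemy.
; Each hit drops a coin; with none left, it spawns a BP_Jobless citizen and a BP_Armor, then destroys itself.
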(event `self.ReceiveBeginPlay`
  (`parent.ReceiveBeginPlay`)
  (`KismetSystemLibrary.Delay` 0.1)
  (`self.SetAIJob`))

(event `/Game/Sihoo/SH_Blueprint/BPS_KingdomTest/Citizen/BPIS_Citizen.OnDamaged`
  (`self.MinusCoin`))

(event `self.ReceiveAnyDamage`
  (params (Damage :type "Float (single-precision)") (DamageType :type "DamageType Object Reference") (InstigatedBy :type "Controller Object Reference") (DamageCauser :type "Actor Object Reference"))
  (`/Game/Sihoo/SH_Blueprint/BPS_KingdomTest/Citizen/BPIS_Citizen.OnDamaged`))

(event `self.AttackRange.OnComponentBeginOverlap`
  (params (OverlappedComponent :type "PrimitiveComponent Object Reference") (OtherActor :type "Actor Object Reference") (OtherComp :type "PrimitiveComponent Object Reference") (OtherBodyIndex :type Integer) (bFromSweep :type Boolean) (SweepResult :type "HitResult Structure (by ref)"))
  (bind _asbp_enemy (cast `/Game/Kingdom3D/Blueprint/Enemy/BP_Enemy` OtherActor))
  (bind _output_get (set `self.enemy` _asbp_enemy))
  (`self.SetEnemyHP` (`/Game/Kingdom3D/Blueprint/Enemy/BP_Enemy.HP` _output_get)))

(event `self.AttackRange.OnComponentEndOverlap`
  (params (OverlappedComponent :type "PrimitiveComponent Object Reference") (OtherActor :type "Actor Object Reference") (OtherComp :type "PrimitiveComponent Object Reference") (OtherBodyIndex :type Integer))
  (`self.SetEnemyHP` 0))

(event `Attack_Event`
  (bind _enemy (`self.enemy`))
  (bind _enemy_2 (`self.enemy`))
  (if (`KismetSystemLibrary.IsValid` _enemy)
    (`/Game/Kingdom3D/Blueprint/Enemy/BP_Enemy.OnDamaged` _enemy)
    (if (`KismetSystemLibrary.IsValid` _enemy_2)
      (`self.SetEnemyHP` (`/Game/Kingdom3D/Blueprint/Enemy/BP_Enemy.HP` _enemy_2)))))

(fn `MinusCoin`
  (locals (VecTmp :type "Vector Structure"))
  (bind _curcoin (`self.curCoin`))
  (bind _returnvalue (`self.GetTransform` self))
  (bind (_returnvalue_location _returnvalue_rotation _returnvalue_scale) (`KismetMathLibrary.BreakTransform` (`self.GetTransform` self)))
  (if (> _curcoin 0)
    (`/Engine/EditorBlueprintResources/StandardMacros.DecrementInt` _curcoin
      (:`  `
        (if (> (.x (.location _returnvalue)) 0.0)
          (`|SpawnActorFromClass` "/Game/Kingdom3D/Blueprint/Item/BP_Coin.BP_Coin_C" (`KismetMathLibrary.MakeTransform` (`KismetMathLibrary.MakeVector` (+ (.x (.location _returnvalue)) 20.0) (.y (.location _returnvalue)) (.z (.location _returnvalue))) (.rotation _returnvalue) (.scale _returnvalue)) "Undefined" "MultiplyWithRoot" null null)
          (else
            (`|SpawnActorFromClass` "/Game/Kingdom3D/Blueprint/Item/BP_Coin.BP_Coin_C" (`KismetMathLibrary.MakeTransform` (`KismetMathLibrary.MakeVector` (- (.x (.location _returnvalue)) 20.0) (.y (.location _returnvalue)) (.z (.location _returnvalue))) (.rotation _returnvalue) (.scale _returnvalue)) "Undefined" "MultiplyWithRoot" null null)))
        (return)))
    (else
      (`AIBlueprintHelperLibrary.SpawnAIFromClass` "/Game/Kingdom3D/Blueprint/Citizen/Jobless/BP_Jobless.BP_Jobless_C" "/Game/Kingdom3D/Blueprint/Citizen/AI/BT_Citizen.BT_Citizen" _returnvalue_location _returnvalue_rotation false null)
      (bind _output_get (set `local.VecTmp` _returnvalue_location))
      (`|SpawnActorFromClass` "/Game/Kingdom3D/Blueprint/Item/BP_Armor.BP_Armor_C" (`KismetMathLibrary.MakeTransform` (`KismetMathLibrary.MakeVector` (+ (.x _output_get) 20.0) (.y _output_get) (.z _output_get)) _returnvalue_rotation _returnvalue_scale) "Undefined" "MultiplyWithRoot" null null)
      (`self.K2_DestroyActor`)
      (return))))

(fn `SetAIJob`
  (bind _asai_citizen (cast `/Game/Kingdom3D/Blueprint/Citizen/AI/AI_Citizen` (`AIBlueprintHelperLibrary.GetAIController` self))
    (:`then`
      (set `/Game/Kingdom3D/Blueprint/Citizen/AI/AI_Citizen.Knight` self _asai_citizen)
      (bind _output_get (set `/Game/Kingdom3D/Blueprint/Citizen/AI/AI_Citizen.Job` "NewEnumerator5" _asai_citizen))
      (`BlackboardComponent.SetValueAsEnum` (`AIController.Blackboard` _asai_citizen) "Job" _output_get))
    (:`CastFailed`
      (`KismetSystemLibrary.PrintString` "CastFailed"))))

(fn `SetEnemyHP`
  (params (Enemy :type Integer))
  (`BlackboardComponent.SetValueAsInt` (`AIBlueprintHelperLibrary.GetBlackboard` (`AIBlueprintHelperLibrary.GetAIController` self)) "EnemyHP" Enemy))

(fn `UserConstructionScript`
  (`parent.UserConstructionScript`))