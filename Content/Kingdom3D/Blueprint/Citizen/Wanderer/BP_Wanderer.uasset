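; BP_Wanderer is a citizen pawn that becomes a Jobless citizen when it touches a coin.
; Shortly after BeginPlay, it registers itself with its AI_Citizen controller and writes the first job enum value to the controller and its Blackboard.
; On coin overlap, it destroys the coin, spawns BP_Jobless running BT_Citizen at its own transform, then destroys itself, so promotion works by replacing the pawn.
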(event `self.ReceiveBeginPlay`
  (`parent.ReceiveBeginPlay`)
  (`KismetSystemLibrary.Delay` 0.1)
  (`self.SetAIJob`))

(event `self.Collision.OnComponentBeginOverlap`
  (params (OverlappedComponent :type "PrimitiveComponent Object Reference") (OtherActor :type "Actor Object Reference") (OtherComp :type "PrimitiveComponent Object Reference") (OtherBodyIndex :type Integer) (bFromSweep :type Boolean) (SweepResult :type "HitResult Structure (by ref)"))
  (bind (_returnvalue_location _returnvalue_rotation) (`KismetMathLibrary.BreakTransform` (`self.GetTransform` self)))
  (bind _asbp_coin (cast `/Game/Kingdom3D/Blueprint/Item/BP_Coin` OtherActor))
  ;[1 1 1] Upgrade to Jobless
  (`self.K2_DestroyActor` _asbp_coin)
  (`AIBlueprintHelperLibrary.SpawnAIFromClass` "/Game/Kingdom3D/Blueprint/Citizen/Jobless/BP_Jobless.BP_Jobless_C" "/Game/Kingdom3D/Blueprint/Citizen/AI/BT_Citizen.BT_Citizen" _returnvalue_location _returnvalue_rotation false null)
  (`self.K2_DestroyActor`))

(fn `SetAIJob`
  (bind _asai_citizen (cast `/Game/Kingdom3D/Blueprint/Citizen/AI/AI_Citizen` (`AIBlueprintHelperLibrary.GetAIController` self))
    (:`then`
      (set `/Game/Kingdom3D/Blueprint/Citizen/AI/AI_Citizen.Wanderer` self _asai_citizen)
      (bind _output_get (set `/Game/Kingdom3D/Blueprint/Citizen/AI/AI_Citizen.Job` "NewEnumerator0" _asai_citizen))
      (`BlackboardComponent.SetValueAsEnum` (`AIController.Blackboard` _asai_citizen) "Job" _output_get))
    (:`CastFailed`
      (`KismetSystemLibrary.PrintString` "CastFailed"))))

(fn `UserConstructionScript`
  (`parent.UserConstructionScript`))