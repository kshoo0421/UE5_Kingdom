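; BP_Carpenter is the carpenter citizen character, which registers its job with its AI controller and reacts to damage.
; Shortly after BeginPlay it casts its controller to AI_Citizen, assigns itself as Carpenter and writes the job enum to the Blackboard.
; Any damage makes it drop a coin; with none left, it drops a BP_Hammer and replaces itself with a jobless citizen.
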(event `self.ReceiveBeginPlay`
  ;[1 1 1] Begin Play : Set AI Job
  (`parent.ReceiveBeginPlay`)
  (`KismetSystemLibrary.Delay` 0.1)
  (`self.SetAIJob`))

(event `/Game/Sihoo/SH_Blueprint/BPS_KingdomTest/Citizen/BPIS_Citizen.OnDamaged`
  (`self.MinusCoin`))

(event `self.ReceiveAnyDamage`
  (params (Damage :type "Float (single-precision)") (DamageType :type "DamageType Object Reference") (InstigatedBy :type "Controller Object Reference") (DamageCauser :type "Actor Object Reference"))
  (`/Game/Sihoo/SH_Blueprint/BPS_KingdomTest/Citizen/BPIS_Citizen.OnDamaged`))

(fn `Drop Item`
  (bind _returnvalue (`self.GetTransform` self))
  ;[1 1 1] Drop Hammer
  (`|SpawnActorFromClass` "/Game/Kingdom3D/Blueprint/Item/BP_Hammer.BP_Hammer_C" (`KismetMathLibrary.MakeTransform` (`KismetMathLibrary.MakeVector` (+ (.x (.location _returnvalue)) 20.0) (.y (.location _returnvalue)) (.z (.location _returnvalue))) (.rotation _returnvalue) (.scale _returnvalue)) "Undefined" "MultiplyWithRoot" null null)
  (return))

(fn `MinusCoin`
  (locals (VecTmp :type "Vector Structure"))
  ;[1 1 1] Minus Coin
  ;;[1 0.5 1] If CurCoin > 0
  (if (> (`self.curCoin`) 0)
    ;;[1 0.5 1] Drop Coin
    (`self.Drop Coin`)
    (else
      ;;[1 0.5 1] Character Die
      (`self.Drop Item`)
      (`self.SpawnJoblessInsteadSelf`)))
  (return))

(fn `SetAIJob`
  ;[1 1 1] Set AI Job
  ;;[1 0.5 1] AI Controller를 AI Citizen으로 Cast
  (bind _asai_citizen (cast `/Game/Kingdom3D/Blueprint/Citizen/AI/AI_Citizen` (`AIBlueprintHelperLibrary.GetAIController` self))
    (:`then`
      ;;[1 0.5 1] Set Caroebter in Controller
      (set `/Game/Kingdom3D/Blueprint/Citizen/AI/AI_Citizen.Carpenter` self _asai_citizen)
      (bind _output_get (set `/Game/Kingdom3D/Blueprint/Citizen/AI/AI_Citizen.Job` "NewEnumerator3" _asai_citizen))
      (`BlackboardComponent.SetValueAsEnum` (`AIController.Blackboard` _asai_citizen) "Job" _output_get)
      (return))
    (:`CastFailed`
      ;;[1 0.5 1] Cast Failed : Error
      (`KismetSystemLibrary.PrintString` "CastFailed"))))

(fn `UserConstructionScript`
  (`parent.UserConstructionScript`))