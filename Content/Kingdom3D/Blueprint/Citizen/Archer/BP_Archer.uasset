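; Archer citizen character that attacks enemies and animals and registers itself and its job with the AI_Citizen controller shortly after BeginPlay.
; An attack-range overlap caches the target and mirrors its HP to the blackboard, which Attack_Event refreshes after damaging it.
; When damaged, it drops a coin or, with none left, drops a bow and is replaced by a jobless citizen.
; Day-state and last-wall blackboard setters are unfinished.
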(event `self.ReceiveBeginPlay`
  ;[1 1 1] Begin Play : Set AI Job
  (`parent.ReceiveBeginPlay`)
  (`KismetSystemLibrary.Delay` 0.1)
  (`self.Set AIJob`))

(event `self.AttackRange.OnComponentBeginOverlap`
  (params (OverlappedComponent :type "PrimitiveComponent Object Reference") (OtherActor :type "Actor Object Reference") (OtherComp :type "PrimitiveComponent Object Reference") (OtherBodyIndex :type Integer) (bFromSweep :type Boolean) (SweepResult :type "HitResult Structure (by ref)"))
  (bind _asbp_enemy (cast `/Game/Kingdom3D/Blueprint/Enemy/BP_Enemy` OtherActor)
    (:`then`
      (bind _output_get (set `self.enemy` _asbp_enemy))
      (`self.SetBBEnemyHP` (`/Game/Kingdom3D/Blueprint/Enemy/BP_Enemy.HP` _output_get)))
    (:`CastFailed`
      (bind _asbpn_animal (cast `/Game/Nyeong/NY_BluePrint/Animal/BPN_Animal` OtherActor))
      (bind _output_get_2 (set `self.animal` _asbpn_animal))
      (`self.SetBBEnemyHP` (`/Game/Nyeong/NY_BluePrint/Animal/BPN_Animal.Hp` _output_get_2)))))

(event `self.AttackRange.OnComponentEndOverlap`
  (params (OverlappedComponent :type "PrimitiveComponent Object Reference") (OtherActor :type "Actor Object Reference") (OtherComp :type "PrimitiveComponent Object Reference") (OtherBodyIndex :type Integer))
  (`self.SetBBEnemyHP` 0))

(event `Attack_Event`
  (bind _enemy (`self.enemy`))
  (bind _enemy_2 (`self.enemy`))
  (bind _animal (`self.animal`))
  (if (`KismetSystemLibrary.IsValid` _enemy)
    (`/Game/Kingdom3D/Blueprint/Enemy/BP_Enemy.OnDamaged` _enemy)
    (if (`KismetSystemLibrary.IsValid` _enemy_2)
      (`self.SetBBEnemyHP` (`/Game/Kingdom3D/Blueprint/Enemy/BP_Enemy.HP` _enemy_2))
      (else
        (`self.SetBBEnemyHP` 0 :!label _label)))
    (else
      (`/Game/Nyeong/NY_BluePrint/Animal/BPN_Animal.On Damaged` (`self.animal`))
      (if (`KismetSystemLibrary.IsValid` _animal)
        (`self.SetBBEnemyHP` (`/Game/Nyeong/NY_BluePrint/Animal/BPN_Animal.Hp` _animal))
        (else
          (goto _label))))))

(event `/Game/Sihoo/SH_Blueprint/BPS_KingdomTest/Citizen/BPIS_Citizen.OnDamaged`
  (`self.MinusCoin`))

(event `self.ReceiveAnyDamage`
  (params (Damage :type "Float (single-precision)") (DamageType :type "DamageType Object Reference") (InstigatedBy :type "Controller Object Reference") (DamageCauser :type "Actor Object Reference"))
  (`/Game/Sihoo/SH_Blueprint/BPS_KingdomTest/Citizen/BPIS_Citizen.OnDamaged`))

(fn `Drop Item`
  (bind _returnvalue (`self.GetTransform` self))
  ;[1 1 1] Drop Bow
  (`|SpawnActorFromClass` "/Game/Kingdom3D/Blueprint/Item/BP_Bow.BP_Bow_C" (`KismetMathLibrary.MakeTransform` (`KismetMathLibrary.MakeVector` (+ (.x (.location _returnvalue)) 20.0) (.y (.location _returnvalue)) (.z (.location _returnvalue))) (.rotation _returnvalue) (.scale _returnvalue)) "Undefined" "MultiplyWithRoot" null null)
  (return))

(fn `MinusCoin`
  ;[1 1 1] Minus Coin
  ;;[1 0.5 1] If CurCoin > 0
  (if (> (`self.curCoin`) 0)
    ;;[1 0.5 1] Drop Coin
    (`self.Drop Coin`)
    (else
      ;;[1 0.5 1] Character Die
      (`self.Drop Item`)
      (`self.SpawnJoblessInsteadSelf`)))
  (return))

(fn `Set AIJob`
  ;[1 1 1] Set AI Job
  ;;[1 0.5 1] AI Controller를 AI Citizen으로 Cast
  (bind _asai_citizen (cast `/Game/Kingdom3D/Blueprint/Citizen/AI/AI_Citizen` (`AIBlueprintHelperLibrary.GetAIController` self))
    (:`then`
      ;;[1 0.5 1] Set Archer in Controller
      (set `/Game/Kingdom3D/Blueprint/Citizen/AI/AI_Citizen.Archer` self _asai_citizen)
      (bind _output_get (set `/Game/Kingdom3D/Blueprint/Citizen/AI/AI_Citizen.Job` "NewEnumerator2" _asai_citizen))
      (`BlackboardComponent.SetValueAsEnum` (`AIController.Blackboard` _asai_citizen) "Job" _output_get)
      (return))
    (:`CastFailed`
      ;;[1 0.5 1] Cast Failed : Error
      (`KismetSystemLibrary.PrintString` "CastFailed"))))

(fn `SetBBEnemyHP`
  (params (EnemyHP :type Integer))
  ;[1 1 1] Set Enemy HP in Blackboard
  ;;[1 0.5 1] Set Value
  (`BlackboardComponent.SetValueAsInt` (`AIBlueprintHelperLibrary.GetBlackboard` (`AIBlueprintHelperLibrary.GetAIController` self)) "EnemyHP" EnemyHP))

(fn `SetDayState`
  (locals (DayManager :type "/Game/Kingdom3D/Blueprint/Manager/ChildManagers/BP_DayManager Object Reference") (DayState :type "/Game/Kingdom3D/Blueprint/Manager/EN_DayState Enum"))
  ;[1 1 1] 미완 - daymanager/state 받아와야함
  (`BlackboardComponent.SetValueAsEnum` (`AIBlueprintHelperLibrary.GetBlackboard` (`AIBlueprintHelperLibrary.GetAIController` self)) "DayState" (`local.DayState`)))

(fn `SetLastWall`
  ;[1 1 1] 미완 - terrainmanager/state 받아와야함
  (`BlackboardComponent.SetValueAsVector` (`AIBlueprintHelperLibrary.GetBlackboard` (`AIBlueprintHelperLibrary.GetAIController` self)) "LastWall" (0.0 0.0 0.0)))

(fn `UserConstructionScript`
  (`parent.UserConstructionScript`))