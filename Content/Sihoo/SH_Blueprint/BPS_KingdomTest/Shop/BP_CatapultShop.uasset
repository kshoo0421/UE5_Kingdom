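; BP_CatapultShop is a skeleton for a catapult shop in the KingdomTest area, with no working logic yet.
; It declares functions to produce, destroy and take catapults (Ctp) per left or right side, plus queries for whether a side's catapult is on and whether items are maxed.
; The action functions are empty, both queries return false, and BeginPlay, overlap and Tick events are disabled.
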(fn `DestroyCtp`
  (params (isLeft :type Boolean)))

(fn `GetIsCtpOn`
  (params (isLeft :type Boolean))
  (returns (result :type Boolean))
  (return false))

(fn `IsItemMax`
  (returns (result :type Boolean))
  (return false))

(fn `ProduceCtp`
  (params (isLeft :type Boolean)))

(fn `TakeCtp`
  (params (isLeft :type Boolean)))

(fn `UserConstructionScript`
  (`parent.UserConstructionScript`))