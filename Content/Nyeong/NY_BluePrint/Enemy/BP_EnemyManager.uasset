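; Enemy manager that spawns waves of enemies and makes them run away, subscribing to the DayManager's day-start and night-start events.
; Spawning picks the left portal on even days and the right on odd days, then creates one enemy per day number with a delayed loop.
; Each enemy records its portal and joins a tracked array, which the run-away event uses to switch every enemy's state.
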(event `self.ReceiveBeginPlay`
  (bind _output_get (set `self.DayManager` (`Actor.GetComponentByClass` (`self.ManagerActor`) "/Game/Kingdom3D/Blueprint/Manager/BP_DayManager.BP_DayManager_C")))
  (add `/Game/Kingdom3D/Blueprint/Manager/BP_DayManager.DayStartEvent` _output_get (`|CreateDelegate` :!event `MakeEnemysRunAway`))
  (add `/Game/Kingdom3D/Blueprint/Manager/BP_DayManager.NightStartEvent` _output_get (`|CreateDelegate` :!event `SpawnEnemys`)))

(event `MakeEnemysRunAway`
  (for _array_element (`self.Enemys`)
    (set `/Game/Nyeong/NY_BluePrint/Enemy/BPN_Enemy.state` "NewEnumerator3" _array_element)
    (`KismetSystemLibrary.PrintString` "MakeRunAway")))

(event `SpawnEnemys`
  (bind _day (`/Game/Kingdom3D/Blueprint/Manager/BP_DayManager.day` (`self.DayManager`)))
  (if (== (mod _day 2) 0)
    (set `self.curSpawnPortal` (`self.LeftPortal`))
    (else
      (set `self.curSpawnPortal` (`self.RightPortal`))))
  (`/Game/Kingdom3D/Blueprint/Additional/ForLoopWithDelay.ForLoopWithDelay` 1 _day 1.0
    (:`LoopBody`
      (bind _returnvalue (`|SpawnActorFromClass` "/Game/Nyeong/NY_BluePrint/Enemy/BPN_Enemy.BPN_Enemy_C" (`Actor.GetTransform` (`self.curSpawnPortal`)) "AdjustIfPossibleButAlwaysSpawn" "MultiplyWithRoot" null null))
      (set `/Game/Nyeong/NY_BluePrint/Enemy/BPN_Enemy.spawnPortal` (`self.curSpawnPortal`) _returnvalue)
      (`KismetArrayLibrary.Array_Add` (`self.Enemys`) _returnvalue))))